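; Demo actor from the horse starter kit that moves as either a horse or a car via a projectile movement component, repeatedly restarting from its spawn point.
; The construction script uses the Type enum to show the matching mesh, set audio volume (muted for the horse), speed and reset delay, with the car faster and looping sooner.
; On BeginPlay it stores its location, and a looping timer snaps it back there.
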(event Custom|ResetLoc
  (Transformation|SetActorLocation (Variables|Default|GetStartLoc) false false))

(event EventBeginPlay
  (Variables|Default|SetStartLoc (Transformation|GetActorLocation))
  (Utilities|Time|SetTimerbyEvent (delegate Custom|ResetLoc) (Variables|Default|GetDelayTime) true))

(fn ConstructionScript
  (bind _projectilemovement (Variables|Default|GetProjectileMovement))
  (bind _projectilemovement_2 (Variables|Default|GetProjectileMovement))
  (switch Utilities|FlowControl|Switch|SwitchonMovable_Type (Variables|Default|GetType)
    (:NewEnumerator0
      (Rendering|SetVisibility (Variables|SkeletalMeshActor|GetSkeletalMeshComponent) true false)
      (Rendering|SetVisibility (Variables|Default|GetCube) false false)
      (Audio|Components|Audio|SetVolumeMultiplier (Variables|Default|GetAudio) 0.0 :!class /Script/Engine.AudioComponent)
      (Variables|/Script/Engine.ProjectileMovementComponent|SetInitialSpeed _projectilemovement_2 1.5e+03)
      (Variables|/Script/Engine.ProjectileMovementComponent|SetMaxSpeed _projectilemovement_2 1.5e+03)
      (Variables|Default|SetDelayTime 6.5))
    (:NewEnumerator1
      (Rendering|SetVisibility (Variables|SkeletalMeshActor|GetSkeletalMeshComponent) false false)
      (Rendering|SetVisibility (Variables|Default|GetCube) true false)
      (Audio|Components|Audio|SetVolumeMultiplier (Variables|Default|GetAudio) 1.0 :!class /Script/Engine.AudioComponent)
      (Variables|/Script/Engine.ProjectileMovementComponent|SetInitialSpeed _projectilemovement 5e+03)
      (Variables|/Script/Engine.ProjectileMovementComponent|SetMaxSpeed _projectilemovement 5e+03)
      (Variables|Default|SetDelayTime 2.0))))