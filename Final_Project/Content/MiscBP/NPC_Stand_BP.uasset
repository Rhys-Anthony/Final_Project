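; An interactable NPC stand that highlights and plays dialogue for the player character.
; On BeginPlay it caches the skeleton knight girl NPC and the Main_Char player.
; Its overlap sphere swaps the mesh to an orange material and scales the NPC up while the player is inside, reverting on exit.
; Interact, guarded against re-entry, plays a dialogue sound above the stand and switches the player to the NPC camera for a few seconds.
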(event OnComponentBeginOverlap(Sphere)
  (params (OverlappedComponent :type Primitive%20Component%20Object%20Reference) (OtherActor :type Actor%20Object%20Reference) (OtherComp :type Primitive%20Component%20Object%20Reference) (OtherBodyIndex :type Integer) (bFromSweep :type Boolean) (SweepResult :type Hit%20Result%20Structure%20%28by%20ref%29))
  (if (== (Utilities|GetClass OtherActor) "/Game/ThirdPerson/Blueprints/Main_Char.Main_Char_C")
    (Rendering|Material|SetMaterial (Variables|Debug|GetStaticMeshComponent) 0 "/Game/Mats/Orange_Inst_MI.Orange_Inst_MI")
    (Default|ScaleUp (Variables|Default|GetNPC_Ref))))

(event OnComponentEndOverlap(Sphere)
  (params (OverlappedComponent :type Primitive%20Component%20Object%20Reference) (OtherActor :type Actor%20Object%20Reference) (OtherComp :type Primitive%20Component%20Object%20Reference) (OtherBodyIndex :type Integer))
  (if (== (Utilities|GetClass OtherActor) "/Game/ThirdPerson/Blueprints/Main_Char.Main_Char_C")
    (Rendering|Material|SetMaterial (Variables|Debug|GetStaticMeshComponent) 0 "/Engine/BasicShapes/BasicShapeMaterial.BasicShapeMaterial")
    (Default|ScaleDown (Variables|Default|GetNPC_Ref))))

(event EventInteract
  (bind _returnvalue (Transformation|GetActorLocation))
  (if (not (Variables|Default|GetInteracting?))
    (Variables|Default|SetInteracting? true)
    (Audio|PlaySoundatLocation "/Game/SFX/Sounds/MetaSounds/Dialogue/Dialogue1.Dialogue1" (Math|Vector|MakeVector (.x _returnvalue) (.y _returnvalue) (+ (.z _returnvalue) 5e+01)) "0, 0, 0" 1.0 1.0 0.0 0 0 0 0)
    (Default|NPCCam (Variables|Default|GetPlayer_Ref) true)
    (Utilities|FlowControl|Delay 3.5)
    (Default|NPCCam (Variables|Default|GetPlayer_Ref) false)
    (Variables|Default|SetInteracting? false)))

(event EventBeginPlay
  (bind _returnvalue (Actor|GetActorOfClass "/Game/MiscBP/Another_Skeleton_Knight_Girl_blue_Blueprint.Another_Skeleton_Knight_Girl_blue_Blueprint_C"))
  (Variables|Default|SetNPC_Ref _returnvalue)
  (bind _returnvalue_2 (Actor|GetActorOfClass "/Game/ThirdPerson/Blueprints/Main_Char.Main_Char_C"))
  (Variables|Default|SetPlayer_Ref _returnvalue_2))

(fn ConstructionScript)